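; BP_PersonajeCat is a player-controlled cat character that moves, turns and keeps an orb count.
; On BeginPlay it registers the IMC_PersonajeInput Enhanced Input mapping context with the player controller's subsystem.
; IA_Mirar drives controller yaw only, and IA_Movimiento scales the actor's forward vector, so movement runs only along the facing axis.
; The ObtenerOrbes event updates the Orbes total by addition.
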(event `self.ReceiveBeginPlay`
  (bind _asplayer_controller (cast `PlayerController` (`self.GetController`)))
  (`EnhancedInputSubsystemInterface.AddMappingContext` (pcsubsystem `EnhancedInputLocalPlayerSubsystem` _asplayer_controller) "/Game/Inputs/MapingContext/IMC_PersonajeInput.IMC_PersonajeInput" 0 (struct)))

(event `EnhancedInput|/Game/Inputs/InputActions/IA_Mirar`
  (params (ActionValue :type "Float (double-precision)") (ElapsedSeconds :type "Float (double-precision)") (TriggeredSeconds :type "Float (double-precision)") (InputAction :type "InputAction Object Reference" :default "/Game/Inputs/InputActions/IA_Mirar.IA_Mirar"))
  (:`Triggered`
    (`self.AddControllerYawInput` ActionValue)))

(event `EnhancedInput|/Game/Inputs/InputActions/IA_Movimiento`
  (params (ActionValue :type "Float (double-precision)") (ElapsedSeconds :type "Float (double-precision)") (TriggeredSeconds :type "Float (double-precision)") (InputAction :type "InputAction Object Reference" :default "/Game/Inputs/InputActions/IA_Movimiento.IA_Movimiento"))
  (:`Triggered`
    (`self.AddMovementInput` (* ActionValue (`self.GetActorForwardVector`)))))

(event `/Game/Interfaces/BPI_Recolectar.ObtenerOrbes`
  (params (Orbes :type Integer))
  (set `self.Orbes` (+ Orbes (`self.Orbes`))))

(fn `UserConstructionScript`)