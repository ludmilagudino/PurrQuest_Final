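; BP_Cat is the player cat character for a side-scrolling platformer, using Enhanced Input for movement, look and jump.
; Movement runs along world X, snapping control yaw to face the direction of acceleration.
; Tick teleports it to InitialLocation below a fall height, and an orb event adds to the collected count with message and sound.
; Walking off a ledge sets a timed coyote-time flag, which these graphs never read.
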(event `self.ReceiveBeginPlay`
  (bind _asplayer_controller (cast `PlayerController` (`self.GetController`)))
  (`EnhancedInputSubsystemInterface.AddMappingContext` (pcsubsystem `EnhancedInputLocalPlayerSubsystem` _asplayer_controller) "/Game/Inputs/MapingContext/IMC_PersonajeInput.IMC_PersonajeInput" 0 (struct))
  (`KismetSystemLibrary.PrintString` "Mundo actual: \nAlta Gracia")
  (`GameplayStatics.PlaySound2D` "/Game/SoundEffects/Magic.Magic" 0.2 1.0 0.0 null null))

(event `EnhancedInput|/Game/Inputs/InputActions/IA_Mirar`
  (params (ActionValue :type "Float (double-precision)") (ElapsedSeconds :type "Float (double-precision)") (TriggeredSeconds :type "Float (double-precision)") (InputAction :type "InputAction Object Reference" :default "/Game/Inputs/InputActions/IA_Mirar.IA_Mirar"))
  (:`Triggered`
    (`self.AddControllerYawInput` ActionValue)))

(event `EnhancedInput|/Game/Inputs/InputActions/IA_Movimiento`
  (params (ActionValue :type "Float (double-precision)") (ElapsedSeconds :type "Float (double-precision)") (TriggeredSeconds :type "Float (double-precision)") (InputAction :type "InputAction Object Reference" :default "/Game/Inputs/InputActions/IA_Movimiento.IA_Movimiento"))
  (bind _returnvalue (`self.GetController`))
  (bind _returnvalue_x (`KismetMathLibrary.BreakVector` (`CharacterMovementComponent.GetCurrentAcceleration` (`self.CharacterMovement`))))
  ; Movimiento
  (:`Triggered`
    (`self.AddMovementInput` (1.0 0.0 0.0) ActionValue)
    (`/Engine/EditorBlueprintResources/StandardMacros.CompareFloat` _returnvalue_x
      (:`>`
        (`Controller.SetControlRotation` _returnvalue (`KismetMathLibrary.MakeRotator` 0.0)))
      (:`<`
        (`Controller.SetControlRotation` _returnvalue (`KismetMathLibrary.MakeRotator` 0.0 0.0 180.0))))))

(event `EnhancedInput|/Game/Inputs/InputActions/IA_Saltar`
  (params (ActionValue :type "Float (double-precision)") (ElapsedSeconds :type "Float (double-precision)") (TriggeredSeconds :type "Float (double-precision)") (InputAction :type "InputAction Object Reference" :default "/Game/Inputs/InputActions/IA_Saltar.IA_Saltar"))
  ; Salto
  (:`Started`
    (`self.Jump`)))

(event `self.ReceiveTick`
  (params (DeltaSeconds :type "Float (single-precision)"))
  ; Respawn
  (`self.Respawn`))

(event `/Game/Interfaces/BPI_Recolectar.ObtenerOrbes`
  (params (Orbes :type Integer))
  ; Recoger orbes
  (bind _output_get (set `self.Orbes` (+ Orbes (`self.Orbes`))))
  (`KismetSystemLibrary.PrintString` (`KismetStringLibrary.Concat_StrStr` "Recolectaste un fragmento de paz!  \nTus fragementos actuales son: " (`KismetStringLibrary.Conv_IntToString` _output_get)) true true (struct :`G` 0.66 :`B` 1.0 :`A` 1.0) 5.0)
  (`GameplayStatics.PlaySound2D` "/Game/SoundEffects/Success_1__subtle_.Success_1__subtle_" 0.5 1.0 0.0 null null))

(event `self.OnWalkingOffLedge`
  (params (PreviousFloorImpactNormal :type "Vector Structure (by ref)") (PreviousFloorContactNormal :type "Vector Structure (by ref)") (PreviousLocation :type "Vector Structure (by ref)") (TimeDelta :type "Float (single-precision)"))
  (set `self.IsInCoyoteTime` true)
  (`KismetSystemLibrary.RetriggerableDelay` (`self.CoyoteTime`))
  (set `self.IsInCoyoteTime` false))

(fn `Respawn`
  (bind (_returnvalue_x _returnvalue_y _returnvalue_z) (`KismetMathLibrary.BreakVector` (`self.K2_GetActorLocation`)))
  (if (< _returnvalue_z -1181.0)
    (`self.K2_SetActorLocation` (`self.InitialLocation`))
    (`GameplayStatics.PlaySound2D` "/Game/SoundEffects/Game_Over.Game_Over" 0.5 1.0 0.0 null null)))

(fn `UserConstructionScript`)